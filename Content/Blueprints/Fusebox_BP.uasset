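; Fusebox actor that can be fixed once, reporting its activation to the game manager.
; Interact sets the fixed flag, turns the point light green and calls FuseActivated on the GameManager_BP found at BeginPlay.
; BeginPlay also calls Interact itself after a five-second delay, so the fusebox fixes itself without player input.
; The InteractBox overlap event is empty.
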(event `self.InteractBox.OnComponentBeginOverlap`
  (params (OverlappedComponent :type "PrimitiveComponent Object Reference") (OtherActor :type "Actor Object Reference") (OtherComp :type "PrimitiveComponent Object Reference") (OtherBodyIndex :type Integer) (bFromSweep :type Boolean) (SweepResult :type "HitResult Structure (by ref)")))

(event `Interact`
  (if (not (`self.IsFixed`))
    (set `self.IsFixed` true)
    (`LightComponent.SetLightColor` (`self.PointLight`) (struct :`R` 0.063858 :`G` 1.0 :`A` 1.0) true)
    (`/Game/Blueprints/GameManager_BP.FuseActivated` (`self.GameManager`))))

(event `self.ReceiveBeginPlay`
  (bind _returnvalue (`GameplayStatics.GetActorOfClass` "/Game/Blueprints/GameManager_BP.GameManager_BP_C"))
  (set `self.GameManager` _returnvalue)
  (`KismetSystemLibrary.Delay` 5.0)
  (`self.Interact`))

(fn `UserConstructionScript`)