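; GameManager_BP tracks fuse objectives and whether the player can exit the level.
; On BeginPlay it creates the Objectives_WBP widget, adds it to the viewport and shows the first objective.
; Each FuseActivated event increments the fuse count, shows the matching entry from the Objectives array, and sets CanExit once three fuses are active.
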(event `self.ReceiveBeginPlay`
  (bind _returnvalue (`|CreateWidget` "/Game/UI/Objectives_WBP.Objectives_WBP_C" (`GameplayStatics.GetPlayerController` 0)))
  (bind _output_get (set `self.ObjectivesWidget` _returnvalue))
  (`UserWidget.AddToViewport` _output_get 0)
  (`/Game/UI/Objectives_WBP.SetObjectiveText` (`self.ObjectivesWidget`) (`|GetArrayItem` (`self.Objectives`))))

(event `FuseActivated`
  (bind _result (`/Engine/EditorBlueprintResources/StandardMacros.IncrementInt` (`self.FusesActivated`))
    (:`  `
      (`/Game/UI/Objectives_WBP.SetObjectiveText` (`self.ObjectivesWidget`) (`|GetArrayItem` (`self.Objectives`) _result))
      (if (== (`self.FusesActivated`) 3)
        (set `self.CanExit` true)))))

(fn `UserConstructionScript`)