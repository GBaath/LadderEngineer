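; One segment of an extendable ladder that animates out and in via a timeline and lets interaction retract the parent ladder.
; While the ladder falls, a per-tick box trace stops it and plays an impact sound on hitting anything other than ladder parts or the player.
; An overlap counter on the first-person character disables walking off ledges on shallow-angled ladders, restoring it after the last segment is left.
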(event `self.ReceiveTick`
  (params (DeltaSeconds :type "Float (single-precision)"))
  (`self.FallingIntersectionCheck`))

(event `self.ReceiveBeginPlay`
  (`self.ExtendAnim`))

(event `ExtendAnim`
  (bind (_direction _zpos) (`Timeline|Extend` :!via `PlayFromStart` :!label _label)
    (:`Update`
      _)
    (:`Finished`
      _))
  (`SceneComponent.K2_SetRelativeLocation` (`self.Cube`) (`KismetMathLibrary.MakeVector` 0.0 0.0 _zpos) false false))

(event `RetractAnim`
  (goto _label :!via `ReverseFromEnd`))

(event `self.PlayerChecker.OnComponentBeginOverlap`
  (params (OverlappedComponent :type "PrimitiveComponent Object Reference") (OtherActor :type "Actor Object Reference") (OtherComp :type "PrimitiveComponent Object Reference") (OtherBodyIndex :type Integer) (bFromSweep :type Boolean) (SweepResult :type "HitResult Structure (by ref)"))
  (bind _ladderangle (`/Game/Blueprints/BP_Ladder.LadderAngle` (`self.Ladder`)))
  (bind _asbp_first_person_character (cast `/Game/FirstPerson/Blueprints/BP_FirstPersonCharacter` OtherActor))
  (bind _numsegmentoverlap (`/Game/FirstPerson/Blueprints/BP_FirstPersonCharacter.NumSegmentOverlap` _asbp_first_person_character))
  (`/Engine/EditorBlueprintResources/StandardMacros.IncrementInt` _numsegmentoverlap
    (:`  `
      (if (or (< _ladderangle 45.0) (> _ladderangle 135.0))
        (bind _output_get (set `CharacterMovementComponent.bCanWalkOffLedges` false (`Character.CharacterMovement` _asbp_first_person_character)))
        (`KismetSystemLibrary.PrintString` (`KismetStringLibrary.Conv_BoolToString` _output_get) true true (struct :`R` 0.0847 :`G` 1.0 :`A` 1.0) 2.0 "ssss")
        (`KismetSystemLibrary.PrintString` (`KismetStringLibrary.Conv_IntToString` _numsegmentoverlap) true true (struct :`G` 0.66 :`B` 1.0 :`A` 1.0) 2.0 "aaaaa")))))

(event `self.PlayerChecker.OnComponentEndOverlap`
  (params (OverlappedComponent :type "PrimitiveComponent Object Reference") (OtherActor :type "Actor Object Reference") (OtherComp :type "PrimitiveComponent Object Reference") (OtherBodyIndex :type Integer))
  (bind _asbp_first_person_character (cast `/Game/FirstPerson/Blueprints/BP_FirstPersonCharacter` OtherActor))
  (bind _numsegmentoverlap (`/Game/FirstPerson/Blueprints/BP_FirstPersonCharacter.NumSegmentOverlap` _asbp_first_person_character))
  (bind _result (`/Engine/EditorBlueprintResources/StandardMacros.DecrementInt` _numsegmentoverlap)
    (:`  `
      (if (< _result 1)
        (bind _output_get (set `CharacterMovementComponent.bCanWalkOffLedges` true (`Character.CharacterMovement` _asbp_first_person_character)))
        (`KismetSystemLibrary.PrintString` (`KismetStringLibrary.Conv_BoolToString` _output_get) true true (struct :`R` 0.046794 :`G` 1.0 :`A` 1.0) 2.0 "ssss")
        (`KismetSystemLibrary.PrintString` (`KismetStringLibrary.Conv_IntToString` _numsegmentoverlap) true true (struct :`G` 0.66 :`B` 1.0 :`A` 1.0) 2.0 "aaaaa")))))

(event `/Game/Blueprints/Interact_BPI.Interact`
  (bind _ladder (`self.Ladder`))
  (if (`/Game/Blueprints/BP_Ladder.DoFall` _ladder)
    _
    (elif (not (`/Game/Blueprints/BP_Ladder.IsRetracting` _ladder))
      (`/Game/Blueprints/BP_Ladder.MaxReract` _ladder))))

(fn `FallingIntersectionCheck`
  (bind _box (`self.Box`))
  (bind _returnvalue (`SceneComponent.K2_GetComponentLocation` _box))
  (if (and (`/Game/Blueprints/BP_Ladder.DoFall` (`self.Ladder`)) (`self.DoFallCheck`))
    (bind (_outhit _returnvalue_2) (`KismetSystemLibrary.BoxTraceSingle` _returnvalue _returnvalue (10.0 5.0 10.0) (`SceneComponent.K2_GetComponentRotation` _box) "TraceTypeQuery1" false (`|MakeArray` (`GameplayStatics.GetPlayerPawn` 0) :!type "Actor Object Reference")))
    (if _returnvalue_2
      (bind (_bblockinghit _binitialoverlap _time _distance _location _impactpoint _normal _impactnormal _physmat _hitactor) (`GameplayStatics.BreakHitResult` _outhit))
      (cast `/Game/Blueprints/BP_LadderSegment` _hitactor
        (:`CastFailed`
          (cast `/Game/Blueprints/BP_Ladder` _hitactor
            (:`CastFailed`
              (`/Game/Blueprints/BP_Ladder.StopFall` (`self.Ladder`))
              (`GameplayStatics.PlaySoundAtLocation` "/Game/Audio/LadderImpact.LadderImpact" (`self.K2_GetActorLocation`) (struct) 0.3 (`KismetMathLibrary.RandomFloatInRange` 0.8 1.2) 0.0 "/Game/Audio/Attenuation.Attenuation" null null null))))))))

(fn `GetButtonPromt`
  (returns (Image :type "Texture2D Object Reference") (Prompt :type Text))
  (return null "E"))

(fn `UserConstructionScript`)