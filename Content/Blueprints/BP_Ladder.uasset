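; BP_Ladder is a deployable ladder that extends segment by segment, topples over, and retracts on interaction before hiding itself.
; Extending spawns BP_LadderSegment actors, each attached to the previous one's connection point, with the Top component following the last.
; At maximum extension, Tick rotates the root segment through a curve-driven quaternion slerp, carrying the attached chain.
; Retraction animates and destroys segments from the end on timed DoN loops, with sound.
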(event `UpdateCrankAnim`
  (`SceneComponent.K2_AddRelativeRotation` (`self.Crank`) (struct :`Roll` 1.0) false false))

(event `SpinnCrankAnim`
  (bind _segments (`self.Segments`))
  (`GameplayStatics.PlaySoundAtLocation` "/Game/Audio/crank2.crank2" (`self.K2_GetActorLocation` (`|GetArrayItem` _segments (- (`KismetArrayLibrary.Array_Length` _segments) 1))) (struct) 0.3 (`KismetMathLibrary.RandomFloatInRange` 0.8 1.2) 0.0 "/Game/Audio/Attenuation.Attenuation" null null null))

(event `self.ReceiveBeginPlay`
  (add `self.FinishRetracting` (delegate `OnFinishRetract`)))

(event `OnFinishRetract`
  (`self.SetActorHiddenInGame` true)
  (`self.ResetValues`))

(event `MaxReract`
  (bind _returnvalue (- (`self.NumSegments`) 1))
  ;[0 0.1979 0.03377] FullExtension
  (if (> (`self.NumSegments`) 0)
    (`|ExecutionSequence`
      (:`then_0`
        (`GameplayStatics.PlaySoundAtLocation` "/Game/Audio/Retract.Retract" (`self.K2_GetActorLocation`) (struct) 0.6 (`KismetMathLibrary.RandomFloatInRange` 0.8 1.2) 0.0 "/Game/Audio/Attenuation.Attenuation" null null null)
        (set `self.IsRetracting` true))
      (:`then_1`
        (bind _counter (`/Engine/EditorBlueprintResources/StandardMacros.Do N` _returnvalue :!label _label)
          (:`Exit`
            (`KismetSystemLibrary.Delay` 0.25)
            (`self.DecreaseEvent`)
            (if (== _counter _returnvalue)
              (`|ExecutionSequence`
                (:`then_0`
                  (`KismetSystemLibrary.Delay` 0.22)
                  (`self.FinishRetracting`))
                (:`then_1`
                  (goto _label :!via `Reset`)))
              (else
                (goto _label)))))))
    (else
      (`self.FinishRetracting`))))

(event `self.ReceiveTick`
  (params (DeltaSeconds :type "Float (single-precision)"))
  (bind _segments (`self.Segments`))
  (bind _top (`self.Top`))
  (bind _output (`|GetArrayItem` _segments (- (`KismetArrayLibrary.Array_Length` _segments) 1)))
  (bind _connectionpoint (`/Game/Blueprints/BP_LadderSegment.ConnectionPoint` _output))
  (`|ExecutionSequence`
    (:`then_0`
      ;[0.1719 0.1719 0.1719] LadderTopFollowsLastSegment
      (`/Engine/EditorBlueprintResources/StandardMacros.IsValid` _output
        (:`Is Valid`
          (`SceneComponent.K2_SetWorldLocationAndRotation` _top (`SceneComponent.K2_GetComponentLocation` _connectionpoint) (`SceneComponent.K2_GetComponentRotation` _connectionpoint) false false)
          (`SceneComponent.K2_AddRelativeRotation` _top (struct :`Pitch` 180.0) false false))))
    (:`then_1`
      ;[0.08241 0.08416 0.1615] Fall Logic
      (if (`self.DoFall`)
        (`self.FallingUpdate` (`self.AlphaHolder`))))))

(event `MaxExtend`
  (bind _returnvalue (- (`self.MaxSegments`) 1))
  ;[0 0.1979 0.03377] FullExtension
  (bind _counter (`/Engine/EditorBlueprintResources/StandardMacros.Do N` _returnvalue :!label _label_2)
    (:`Exit`
      (`KismetSystemLibrary.Delay` 0.25)
      (`self.IncreaseEvent`)
      (if (== _counter _returnvalue)
        (`self.Start Falling`)
        (else
          (goto _label_2))))))

(event `IncreaseEvent`
  ;[0.08298 0.2812 0.09673] increasedeecrease
  (`self.Extend`))

(event `DecreaseEvent`
  ;[0.08298 0.2812 0.09673] increasedeecrease
  (`/Engine/EditorBlueprintResources/StandardMacros.DoOnce` false :!label _label_3
    (:`Completed`
      (bind _toremoveafteranim (`self.Decrease`))
      (`KismetSystemLibrary.Delay` 0.2)
      (`self.K2_DestroyActor` _toremoveafteranim)
      (`KismetArrayLibrary.Array_RemoveItem` (`self.Segments`) _toremoveafteranim)
      (goto _label_3 :!via `Reset`))))

(event `ResetValues`
  (set `self.NumSegments` 0)
  (`SceneComponent.K2_SetRelativeLocationAndRotation` (`self.Top`) (0.0 0.0 80.0) (struct :`Yaw` 90.0 :`Roll` 180.0) false true)
  (set `self.IsRetracting` false)
  (set `self.HasFallen` false)
  (set `self.ButtonPrompt` "HOLD"))

(event `/Game/Blueprints/Interact_BPI.Interact`
  (if (`self.DoFall`)
    _
    (elif (not (`self.IsRetracting`))
      (`self.MaxReract`))))

(fn `Decrease`
  (returns (ToRemoveAfterAnim :type "/Game/Blueprints/BP_LadderSegment Object Reference"))
  (bind _segments (`self.Segments`))
  (bind _output (`|GetArrayItem` _segments (- (`KismetArrayLibrary.Array_Length` _segments) 1)))
  (`/Game/Blueprints/BP_LadderSegment.RetractAnim` _output)
  (return _output))

(fn `Extend`
  (locals (`Spawned Segment` :type "/Game/Blueprints/BP_LadderSegment Object Reference"))
  (bind _segments (`self.Segments`))
  (bind _segments_2 (`self.Segments`))
  (bind _output (`|GetArrayItem` _segments (- (`KismetArrayLibrary.Array_Length` _segments) 1)))
  (`/Engine/EditorBlueprintResources/StandardMacros.IncrementInt` (`self.NumSegments`)
    (:`  `
      (`/Engine/EditorBlueprintResources/StandardMacros.IsValid` _output
        (:`Is Valid`
          (`|ExecutionSequence`
            (:`then_0`
              (bind _returnvalue (`|SpawnActorFromClass` "/Game/Blueprints/BP_LadderSegment.BP_LadderSegment_C" (`KismetMathLibrary.MakeTransform` (`SceneComponent.K2_GetComponentLocation` (`/Game/Blueprints/BP_LadderSegment.ConnectionPoint` _output))) "Undefined" "MultiplyWithRoot" null null))
              (`|ExecutionSequence`
                (:`then_0`
                  (set `/Game/Blueprints/BP_LadderSegment.Ladder` self _returnvalue)
                  (`KismetArrayLibrary.Array_Add` (`self.Segments`) _returnvalue))
                (:`then_1`
                  (`self.K2_AttachToActor` _returnvalue (`|GetArrayItem` _segments_2 (- (`KismetArrayLibrary.Array_Length` _segments_2) 2)) "None" "KeepWorld" "KeepRelative" "KeepWorld" true))))
            (:`then_1`
              (`self.SpinnCrankAnim` :!label _label))))
        (:`Is Not Valid`
          (`|ExecutionSequence`
            (:`then_0`
              (`self.InitSegment`))
            (:`then_1`
              (goto _label))))))))

(fn `FallingUpdate`
  (params (RotAlpha :type "Float (double-precision)"))
  (bind _localstartfallrotation (`self.LocalStartFallRotation`))
  (bind _returnvalue (`KismetMathLibrary.FInterpTo_Constant` RotAlpha 1.0 (`GameplayStatics.GetWorldDeltaSeconds`) 0.5))
  (bind _output_get (set `self.AlphaHolder` _returnvalue))
  (`self.K2_SetActorRelativeRotation` (`|GetArrayItem` (`self.Segments`)) (`KismetMathLibrary.Quat_Rotator` (`KismetMathLibrary.Quat_Slerp` (`KismetMathLibrary.Conv_RotatorToQuaternion` _localstartfallrotation) (`KismetMathLibrary.Conv_RotatorToQuaternion` (`KismetMathLibrary.MakeRotator` (+ (.roll _localstartfallrotation) 165.0) (.pitch _localstartfallrotation) (.yaw _localstartfallrotation))) (`CurveFloat.GetFloatValue` (`self.FallingCurve`) _returnvalue))) false false)
  (if (>= _output_get 0.99)
    (`self.StopFall`)))

(fn `GetButtonPromt`
  (returns (Image :type "Texture2D Object Reference") (Prompt :type Text))
  (return "/Game/Graphics/Material/Textures/mouse1.mouse1" (`self.ButtonPrompt`)))

(fn `InitSegment`
  (locals (SpawnedSegment :type "/Game/Blueprints/BP_LadderSegment Object Reference"))
  (bind _returnvalue (`|SpawnActorFromClass` "/Game/Blueprints/BP_LadderSegment.BP_LadderSegment_C" (`KismetMathLibrary.MakeTransform` (`SceneComponent.K2_GetComponentLocation` (`self.Spawnpoint`)) (struct :`Roll` 5.0)) "Undefined" "MultiplyWithRoot" null null))
  (set `local.SpawnedSegment` _returnvalue)
  (`|ExecutionSequence`
    (:`then_0`
      (set `/Game/Blueprints/BP_LadderSegment.Ladder` self (`local.SpawnedSegment`)))
    (:`then_1`
      (`KismetArrayLibrary.Array_Add` (`self.Segments`) (`local.SpawnedSegment`)))
    (:`then_2`
      (`/Engine/EditorBlueprintResources/StandardMacros.IncrementInt` (`self.NumSegments`)))
    (:`then_3`
      (`self.K2_AttachToActor` (`local.SpawnedSegment`) self "None" "KeepWorld" "KeepRelative" "KeepWorld" true))
    (:`then_4`
      (`SceneComponent.K2_SetWorldLocation` (`self.Top`) (`SceneComponent.K2_GetComponentLocation` (`/Game/Blueprints/BP_LadderSegment.ConnectionPoint` (`local.SpawnedSegment`))) false false))))

(fn `Pickup`)

(fn `Start Falling`
  (bind _segments (`self.Segments`))
  (if (not (`self.HasFallen`))
    (if (and (> (`KismetArrayLibrary.Array_Length` _segments) 0) (not (`self.DoFall`)))
      (set `self.LocalStartFallRotation` (`SceneComponent.RelativeRotation` (`/Game/Blueprints/BP_LadderSegment.DefaultSceneRoot` (`|GetArrayItem` _segments))))
      (set `self.DoFall` true)
      (set `self.AlphaHolder` 0.0))))

(fn `StopFall`
  (bind _output (`|GetArrayItem` (`self.Segments`)))
  (bind _returnvalue_roll (`KismetMathLibrary.BreakRotator` (`self.K2_GetActorRotation` _output)))
  (set `self.DoFall` false)
  (set `self.HasFallen` true)
  (if (`KismetSystemLibrary.IsValid` _output)
    (set `self.LadderAngle` _returnvalue_roll)
    (set `self.ButtonPrompt` "E")
    (return)))

(fn `UserConstructionScript`)