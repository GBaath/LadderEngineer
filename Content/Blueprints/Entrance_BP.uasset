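; Entrance actor that acts as the game's exit trigger and shows the ending screen.
; On BeginPlay it finds and caches the GameManager_BP actor.
; When BP_FirstPersonCharacter overlaps its Box while the manager's CanExit is true, it removes all widgets and adds Ending_WBP to the viewport.
; Debug "Hello" prints fire on any overlap and after the ending widget appears.
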(event `self.ReceiveBeginPlay`
  (bind _returnvalue (`GameplayStatics.GetActorOfClass` "/Game/Blueprints/GameManager_BP.GameManager_BP_C"))
  (set `self.GameManager` _returnvalue))

(event `self.Box.OnComponentBeginOverlap`
  (params (OverlappedComponent :type "PrimitiveComponent Object Reference") (OtherActor :type "Actor Object Reference") (OtherComp :type "PrimitiveComponent Object Reference") (OtherBodyIndex :type Integer) (bFromSweep :type Boolean) (SweepResult :type "HitResult Structure (by ref)"))
  (`KismetSystemLibrary.PrintString` "Hello")
  (cast `/Game/FirstPerson/Blueprints/BP_FirstPersonCharacter` OtherActor)
  (if (`/Game/Blueprints/GameManager_BP.CanExit` (`self.GameManager`))
    (`WidgetLayoutLibrary.RemoveAllWidgets`)
    (bind _returnvalue (`|CreateWidget` "/Game/UI/Ending_WBP.Ending_WBP_C" (`GameplayStatics.GetPlayerController` 0)))
    (`UserWidget.AddToViewport` _returnvalue 0)
    (`KismetSystemLibrary.PrintString` "Hello")))

(fn `UserConstructionScript`)