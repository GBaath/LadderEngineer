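; BP_BlinkingLight is a blinking lamp actor that pulses a point light and the glow of its bulb sphere together.
; On BeginPlay it creates a dynamic bulb material, applies the bulb colour to light and material, then waits an initial delay.
; BlinkSpeeds selects one of four macros, each looping its own timeline with a pause between blinks to lerp intensity and glow from zero to their set levels.
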(event `self.ReceiveBeginPlay`
  (bind _sphere (`self.Sphere`))
  ;[1 1 1] Create dynamic material for sphere
  (bind _returnvalue (`PrimitiveComponent.CreateDynamicMaterialInstance` _sphere 0 "/Game/VFX/M_BlinkingLightBulb.M_BlinkingLightBulb" "None"))
  (bind _output_get (set `self.MaterialRef` _returnvalue))
  (`PrimitiveComponent.SetMaterial` _sphere 0 _output_get)
  (set `self.PointLightInitial` (`LightComponentBase.Intensity` (`self.PointLight`)))
  (`LightComponent.SetLightColor` (`self.PointLight`) (`self.BulbColour`) true)
  (`MaterialInstanceDynamic.SetVectorParameterValue` (`self.MaterialRef`) "LampCol" (`self.BulbColour`))
  (`KismetSystemLibrary.Delay` (`self.InitialGlowDelay`))
  (switch `int` (`self.BlinkSpeeds`)
    (:`0`
      (bind (_direction _newtrack_0) (`Timeline|Timeline` :!via `PlayFromStart` :!label _label)
        (:`Update`
          (`LightComponent.SetIntensity` (`self.PointLight`) (`KismetMathLibrary.Lerp` 0.0 (`self.PointLightInitial`) _newtrack_0))
          (`MaterialInstanceDynamic.SetScalarParameterValue` (`self.MaterialRef`) "GlowSTR" (`KismetMathLibrary.Lerp` 0.0 (`self.GlowSTR`) _newtrack_0)))
        (:`Finished`
          (`KismetSystemLibrary.Delay` (`self.GlowDelay`))
          (goto _label :!via `PlayFromStart`))))
    (:`1`
      (bind (_direction_2 _newtrack_0_2) (`Timeline|GlobeHalfSecond` :!via `PlayFromStart` :!label _label_2)
        (:`Update`
          (`LightComponent.SetIntensity` (`self.PointLight`) (`KismetMathLibrary.Lerp` 0.0 (`self.PointLightInitial`) _newtrack_0_2))
          (`MaterialInstanceDynamic.SetScalarParameterValue` (`self.MaterialRef`) "GlowSTR" (`KismetMathLibrary.Lerp` 0.0 (`self.GlowSTR`) _newtrack_0_2)))
        (:`Finished`
          (`KismetSystemLibrary.Delay` (`self.GlowDelay`))
          (goto _label_2 :!via `PlayFromStart`))))
    (:`2`
      (bind (_direction_3 _newtrack_0_3) (`Timeline|BulbTimeline1` :!via `PlayFromStart` :!label _label_3)
        (:`Update`
          (`LightComponent.SetIntensity` (`self.PointLight`) (`KismetMathLibrary.Lerp` 0.0 (`self.PointLightInitial`) _newtrack_0_3))
          (`MaterialInstanceDynamic.SetScalarParameterValue` (`self.MaterialRef`) "GlowSTR" (`KismetMathLibrary.Lerp` 0.0 (`self.GlowSTR`) _newtrack_0_3)))
        (:`Finished`
          (`KismetSystemLibrary.Delay` (`self.GlowDelay`))
          (goto _label_3 :!via `PlayFromStart`))))
    (:`3`
      (bind (_direction_4 _newtrack_0_4) (`Timeline|BulbTimeline` :!via `PlayFromStart` :!label _label_4)
        (:`Update`
          (`LightComponent.SetIntensity` (`self.PointLight`) (`KismetMathLibrary.Lerp` 0.0 (`self.PointLightInitial`) _newtrack_0_4))
          (`MaterialInstanceDynamic.SetScalarParameterValue` (`self.MaterialRef`) "GlowSTR" (`KismetMathLibrary.Lerp` 0.0 (`self.GlowSTR`) _newtrack_0_4)))
        (:`Finished`
          (`KismetSystemLibrary.Delay` (`self.GlowDelay`))
          (goto _label_4 :!via `PlayFromStart`))))))

(fn `UserConstructionScript`)