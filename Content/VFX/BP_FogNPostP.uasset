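; BP_FogNPostP is a VFX actor, named for fog and post-processing, that keeps air dust particles around the player.
; Each tick it moves the AirDust component to the player pawn's location, offset along its velocity by a tunable strength so the dust leads movement.
; On BeginPlay it also forces the game's resolution scale to 40 through Game User Settings, a global side effect.
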(event `self.ReceiveBeginPlay`
  (bind _returnvalue (`GameUserSettings.GetGameUserSettings`))
  (`GameUserSettings.SetResolutionScaleValueEx` _returnvalue 40.0))

(event `self.ReceiveTick`
  (params (DeltaSeconds :type "Float (single-precision)"))
  (bind _returnvalue (`GameplayStatics.GetPlayerPawn` 0))
  (`SceneComponent.K2_SetWorldLocation` (`self.AirDust`) (+ (`self.K2_GetActorLocation` _returnvalue) (* (`self.GetVelocity` _returnvalue) (`self.PartVelocityOffsetSTR`))) false false))

(fn `UserConstructionScript`)